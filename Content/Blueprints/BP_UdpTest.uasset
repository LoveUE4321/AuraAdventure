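; BP_UdpTest is a test Blueprint that exercises a UDPNetwork component for sending and receiving UDP data.
; On BeginPlay it hands its Camera to the component and binds handlers for string and raw data events, then disconnects on EndPlay.
; The handlers print the received string or the sender address, and pressing E sends a fixed test string.
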(event Custom|OnUDPDataRecv
  (params (Data :type String))
  (Development|PrintString Data))

(event Custom|OnUDPRawDataRecv
  (params (Data :type Array%20of%20Bytes) (FromAddress :type String))
  (Development|PrintString FromAddress))

(event EventBeginPlay
  (bind _udpnetwork (Variables|Default|GetUDPNetwork))
  (Class|UDPNetworkComponent|SetCurrentCamera (Variables|Default|GetUDPNetwork) (Variables|Default|GetCamera))
  (EventDispatchers|BindEventtoOnDataReceived _udpnetwork (delegate Custom|OnUDPDataRecv))
  (EventDispatchers|BindEventtoOnRawDataReceived _udpnetwork (delegate Custom|OnUDPRawDataRecv)))

(event EventTick
  (params (DeltaSeconds :type Float%20%28single-precision%29)))

(event EventEndPlay
  (params (EndPlayReason :type EEndPlayReason%20Enum :default "Destroyed"))
  (Class|UDPNetworkComponent|Disconnect (Variables|Default|GetUDPNetwork)))

(event Input|KeyboardEvents|E
  (params (Key :type Key%20Structure :default "None"))
  (:Pressed
    (Class|UDPNetworkComponent|SendString (Variables|Default|GetUDPNetwork) "Send To Udp")))

(fn ConstructionScript)