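; BP_UdpMgr is a UDP manager Blueprint that initializes a socket client UDP receiver on localhost at BeginPlay.
; Separate test chains create a named UDP socket with target and self ports, send messages, and receive them, printing each result to screen.
; These chains have no event driving them, so only the receiver initialization runs; Tick is empty.
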(event EventBeginPlay
  (Class|SocketClientBPLibrary|SocketClientInitUDPReceiver "127.0.0.1" "E_ipv4" 8888 "E_SAB" 65507))

(event EventTick
  (params (DeltaSeconds :type Float%20%28single-precision%29)))

(event Input|KeyboardEvents|E
  (params (Key :type Key%20Structure :default "None")))

(fn ConstructionScript)